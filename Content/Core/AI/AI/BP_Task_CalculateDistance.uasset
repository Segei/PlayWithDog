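; Behavior tree task that measures how far the controlled runner character is from its target along a path.
; It reads the target actor from a blackboard key, gets the path length between both locations and stores it in the RunnerCharacter's Distance.
; It fails on a missing target or invalid pawn, but never finishes if the pawn is not a RunnerCharacter.
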(event EventReceiveExecuteAI
  (params (OwnerController :type AI%20Controller%20Object%20Reference) (ControlledPawn :type Pawn%20Object%20Reference))
  (Variables|Default|SetOwner%20Controller OwnerController)
  (Variables|Default|SetControlled%20Pawn ControlledPawn)
  (bind _asactor (Utilities|Casting|CastToActor (AI|Components|Blackboard|GetValueasObject (AI|GetBlackboard (Variables|Default|GetOwner%20Controller)) (.SelectedKeyName (Utilities|Struct|BreakBlackboardKeySelector (Variables|Default|GetTargetActor)))))
    (:then
      (Variables|Default|SetTarget _asactor)
      (bind _controlled_pawn (Variables|Default|GetControlled%20Pawn)
        (:then
          (bind _asrunner_character (Utilities|Casting|CastToRunnerCharacter _controlled_pawn))
          (Variables|/Script/PlayWithDog.RunnerCharacter|SetDistance _asrunner_character (.PathLength (Class|NavigationSystemV1|GetPathLength (Transformation|GetActorLocation (Variables|Default|GetControlled%20Pawn)) (Transformation|GetActorLocation (Variables|Default|GetTarget)) 0 0)))
          (AI|BehaviorTree|FinishExecute true))
        (:else
          (AI|BehaviorTree|FinishExecute false :!label _label))))
    (:CastFailed
      (goto _label))))