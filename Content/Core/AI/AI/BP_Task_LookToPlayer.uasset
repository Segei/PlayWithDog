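; Behavior tree task that turns the AI pawn to face the nearest player pawn.
; It scans the player pawns from BP_PWDGameMode, keeping the closest under the stored distance threshold, which shrinks with each match and is not reset here.
; One yaw-only RInterpTo step toward the watched pawn finishes the task successfully; having no valid watched pawn fails it.
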(event EventReceiveExecuteAI
  (params (OwnerController :type AI%20Controller%20Object%20Reference) (ControlledPawn :type Pawn%20Object%20Reference))
  (Variables|Default|SetOwner%20Controller OwnerController)
  (Variables|Default|SetControlled%20Pawn ControlledPawn)
  (Variables|Default|GetControlled%20Pawn
    (:then
      (bind _asbp_pwdgame_mode (Utilities|Casting|CastToBP_PWDGameMode (Game|GetGameMode)))
      (bind _returnvalue (Class|PWDGameMode|GetPlayerPawn _asbp_pwdgame_mode))
      (for _array_element _returnvalue
        (Utilities|IsValid _array_element
          (:Is%20Valid
            (bind _controlled_pawn (Variables|Default|GetControlled%20Pawn)
              (:then
                (if (< (Math|Vector|VectorLength (- (Transformation|GetActorLocation _controlled_pawn) (Transformation|GetActorLocation _array_element))) (Variables|Default|GetLenght))
                  (Variables|Default|SetWatchingPawn _array_element)
                  (Variables|Default|SetLenght (Math|Vector|VectorLength (- (Transformation|GetActorLocation _controlled_pawn) (Transformation|GetActorLocation _array_element))))))
              (:else)))))
      (Variables|Default|GetWatchingPawn
        (:then
          (bind _controlled_pawn_2 (Variables|Default|GetControlled%20Pawn)
            (:then
              (Transformation|SetActorRotation _controlled_pawn_2 (Math|Rotator|MakeRotator 0.0 0.0 (.yaw (Math|Interpolation|RInterpTo (Transformation|GetActorRotation (Variables|Default|GetControlled%20Pawn)) (Math|Rotator|FindLookatRotation (Transformation|GetActorLocation (Variables|Default|GetControlled%20Pawn)) (Transformation|GetActorLocation (Variables|Default|GetWatchingPawn))) (Utilities|Time|GetWorldDeltaSeconds) 0.0))))
              (AI|BehaviorTree|FinishExecute true))
            (:else
              (AI|BehaviorTree|FinishExecute false :!label _label))))
        (:else
          (goto _label))))
    (:else)))