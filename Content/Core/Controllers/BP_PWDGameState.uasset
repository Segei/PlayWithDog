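; Game state that relays replicated score and end-of-game changes to the player HUD.
; The rep-notify for CurrentScore gets BP_PlayerHUD from player controller 0 and, after validity checks, pushes the score to the main UI's score table widget.
; The EndGame rep-notify calls the same HUD's end-game switch.
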(event EventOnReplicatedUsingEndGame
  (bind _asbp_player_hud (Utilities|Casting|CastToBP_PlayerHUD (HUD|GetHUD (Game|GetPlayerController 0))))
  (Default|SwtchEndGame _asbp_player_hud))

(event EventOnReplicatedUsingCurrentScore
  (bind _asbp_player_hud (Utilities|Casting|CastToBP_PlayerHUD (HUD|GetHUD (Game|GetPlayerController 0))))
  (bind _mainui (Variables|/Game/Core/UI/BP_PlayerHUD.BP_PlayerHUD_C|GetMainUI _asbp_player_hud)
    (:then
      (bind _wbp_scoretable (Variables|/Game/Core/UI/WBP_MainUI.WBP_MainUI_C|GetWBP_ScoreTable _mainui)
        (:then
          (bind _output_get (Variables|Default|SetCurrent%20Score (Variables|Default|GetCurrentScore)))
          (Default|UpdateScore _wbp_scoretable _output_get))
        (:else)))
    (:else)))

(fn ConstructionScript)